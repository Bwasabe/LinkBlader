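; BP_Object_Rock is a breakable rock object in the interaction system that shatters into fragment items.
; Its BreakItem event flags it as broken, then spawns one BP_Item per entry in Fragments, marked as a fracture.
; Each piece starts at the rock mesh's transform and inherits its velocity.
; The rock then calls DropItem with zero velocity and the destroy flag set, and destroys itself.
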(event EventBeginPlay
  (|CallParentFunction) ; This node is disabled and will not be called.\nDrag off pins to build functionality.
)

(event Collision|EventActorBeginOverlap
  (params (OtherActor :type Actor%20Object%20Reference))
  (|CallParentFunction OtherActor) ; This node is disabled and will not be called.\nDrag off pins to build functionality.
)

(event EventTick
  (params (DeltaSeconds :type Float%20%28single-precision%29))
  (|CallParentFunction DeltaSeconds) ; This node is disabled and will not be called.\nDrag off pins to build functionality.
)

(event EventBreakItem
  (Variables|Runtime|SetBroken true)
  (CallFunction|SpawnFragments))

(fn ConstructionScript
  (|CallParentFunction))

(fn SpawnFragments
  (bind _mesh (Variables|Character|GetMesh))
  (for _array_element (Variables|Init|GetFragments)
    (Game|SpawnActorfromClass "/Game/InteractionSystem/Blueprints/Items/Master/BP_Item.BP_Item_C" (Transformation|GetWorldTransform _mesh) "Undefined" 0 _array_element (Transformation|GetComponentVelocity _mesh) true 0))
  (CallFunction|DropItem "0, 0, 0" true)
  (Actor|DestroyActor))